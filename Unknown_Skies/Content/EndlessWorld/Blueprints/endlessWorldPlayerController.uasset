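; Player controller for the endless world game that starts procedural level generation around the player and opens the in-game pause menu.
; BeginPlay initializes the EndlessWorldComponent, which then generates levels around the player.
; Pressing Tab creates the pause menu widget once and reuses it, adds it to the viewport, switches to UI-only input with a visible cursor and pauses the game.
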(event `self.ReceiveBeginPlay`
  ;[1 1 1] Once this event is called, the EndlessWorldComponent will begin to generate levels around the player
  (`/Game/EndlessWorld/Blueprints/EndlessWorldComponent.Initialize Endless World Component` (`self.EndlessWorldComponent`)) ; Call this from your own Player Controller if you like.
)

(event `Key|Tab`
  (params (Key :type "Key Structure"))
  (bind _returnvalue (`GameplayStatics.GetPlayerController` 0))
  (:`Pressed`
    (`/Engine/EditorBlueprintResources/StandardMacros.IsValid` (`self.InGamePauseMenuRef`)
      (:`Is Valid`
        _)
      (:`Is Not Valid`
        (bind _returnvalue_2 (`|CreateWidget` "/Game/DZG_MenuSystemV1/UI/WBP_InGamePauseMenu.WBP_InGamePauseMenu_C" _returnvalue))
        (bind _output_get (set `self.InGamePauseMenuRef` _returnvalue_2))))
    (`UserWidget.AddToViewport` _output_get 0)
    (`WidgetBlueprintLibrary.SetInputMode_UIOnlyEx` _returnvalue null)
    (set `PlayerController.bShowMouseCursor` true _returnvalue)
    (`GameplayStatics.SetGamePaused` true)))

(fn `UserConstructionScript`)