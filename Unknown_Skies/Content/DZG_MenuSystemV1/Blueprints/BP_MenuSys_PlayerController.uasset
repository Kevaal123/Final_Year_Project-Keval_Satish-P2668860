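; Player controller for the menu system, driving character movement and opening the in-game pause menu.
; Rebindable input axes, split per direction, move the character relative to control yaw; Jump works, while the other actions only print placeholder strings.
; Tab creates or reuses WBP_InGamePauseMenu, switches to UI-only input with cursor, and pauses the game.
; A custom event initializes EndlessWorldComponent; BeginPlay is empty, leaving PlayerCharacterRef unassigned here.
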(event `self.ReceiveBeginPlay`
  ;[0 1 0] SELECT BP_MenuSys_PlayerController in the applicable GameMode. The IA_Menusys_(action/axis) input mappings matche those in the Project's Input Settings.
  ; At BeginPlay, get a reference to the Player Character
)

(event `InputAxis|IA_MenuSys_MoveForward`
  (params (AxisValue :type "Float (single-precision)"))
  (bind _playercharacterref (`self.PlayerCharacterRef`))
  (bind (_returnvalue_roll _returnvalue_pitch _returnvalue_yaw) (`KismetMathLibrary.BreakRotator` (`Pawn.GetControlRotation` _playercharacterref)))
  ;[0 1 0] Input Axis Movement Functions - Forward/Backward and Right/Left were separated to simplify key binding changes
  (`Pawn.AddMovementInput` _playercharacterref (`KismetMathLibrary.GetForwardVector` (`KismetMathLibrary.MakeRotator` 0.0 0.0 _returnvalue_yaw)) AxisValue false))

(event `InputAxis|IA_MenuSys_MoveBackward`
  (params (AxisValue :type "Float (single-precision)"))
  (bind _playercharacterref (`self.PlayerCharacterRef`))
  (bind (_returnvalue_roll _returnvalue_pitch _returnvalue_yaw) (`KismetMathLibrary.BreakRotator` (`Pawn.GetControlRotation` _playercharacterref)))
  ;[0 1 0] Input Axis Movement Functions - Forward/Backward and Right/Left were separated to simplify key binding changes
  (`Pawn.AddMovementInput` _playercharacterref (`KismetMathLibrary.GetForwardVector` (`KismetMathLibrary.MakeRotator` 0.0 0.0 _returnvalue_yaw)) AxisValue false))

(event `CustomEvent`
  ;[1 1 1] Once this event is called, the EndlessWorldComponent will begin to generate levels around the player
  (`/Game/EndlessWorld/Blueprints/EndlessWorldComponent.Initialize Endless World Component` (`self.EndlessWorldComponent`)) ; Call this from your own Player Controller if you like.
)

(event `InputAxis|IA_MenuSys_MoveRight`
  (params (AxisValue :type "Float (single-precision)"))
  (bind _playercharacterref (`self.PlayerCharacterRef`))
  (bind (_returnvalue_roll _returnvalue_pitch _returnvalue_yaw) (`KismetMathLibrary.BreakRotator` (`Pawn.GetControlRotation` _playercharacterref)))
  ;[0 1 0] Input Axis Movement Functions - Forward/Backward and Right/Left were separated to simplify key binding changes
  (`Pawn.AddMovementInput` _playercharacterref (`KismetMathLibrary.GetRightVector` (`KismetMathLibrary.MakeRotator` 0.0 0.0 _returnvalue_yaw)) AxisValue false))

(event `InputAxis|IA_MenuSys_MoveLeft`
  (params (AxisValue :type "Float (single-precision)"))
  (bind _playercharacterref (`self.PlayerCharacterRef`))
  (bind (_returnvalue_roll _returnvalue_pitch _returnvalue_yaw) (`KismetMathLibrary.BreakRotator` (`Pawn.GetControlRotation` _playercharacterref)))
  ;[0 1 0] Input Axis Movement Functions - Forward/Backward and Right/Left were separated to simplify key binding changes
  (`Pawn.AddMovementInput` _playercharacterref (`KismetMathLibrary.GetRightVector` (`KismetMathLibrary.MakeRotator` 0.0 0.0 _returnvalue_yaw)) AxisValue false))

(event `InputAction|IA_MenuSys_Jump`
  (params (Key :type "Key Structure"))
  (bind _playercharacterref (`self.PlayerCharacterRef`))
  ;[0 1 0] Input Action Functions that can be assigned to different key in the Menu System's Key Binding settings
  (:`Pressed`
    (`Character.Jump` _playercharacterref))
  (:`Released`
    (`Character.StopJumping` _playercharacterref)))

(event `InputAction|IA_MenuSys_Crouch`
  (params (Key :type "Key Structure"))
  ;[0 1 0] Input Action Functions that can be assigned to different key in the Menu System's Key Binding settings
  (:`Pressed`
    (`KismetSystemLibrary.PrintString` "Crouch")))

(event `InputAction|IA_MenuSys_Sprint`
  (params (Key :type "Key Structure"))
  ;[0 1 0] Input Action Functions that can be assigned to different key in the Menu System's Key Binding settings
  (:`Pressed`
    (`KismetSystemLibrary.PrintString` "Sprint")))

(event `InputAction|IA_MenuSys_EnterExit`
  (params (Key :type "Key Structure"))
  ;[0 1 0] Input Action Functions that can be assigned to different key in the Menu System's Key Binding settings
  (:`Pressed`
    (`KismetSystemLibrary.PrintString` "Enter/Exit")))

(event `InputAction|IA_MenuSys_SpecialAbility`
  (params (Key :type "Key Structure"))
  ;[0 1 0] Input Action Functions that can be assigned to different key in the Menu System's Key Binding settings
  (:`Pressed`
    (`KismetSystemLibrary.PrintString` "Special Ability")))

(event `InputAction|IA_MenuSys_Map`
  (params (Key :type "Key Structure"))
  ;[0 1 0] Input Action Functions that can be assigned to different key in the Menu System's Key Binding settings
  (:`Pressed`
    (`KismetSystemLibrary.PrintString` "Map")))

(event `InputAction|IA_MenuSys_Inventory`
  (params (Key :type "Key Structure"))
  ;[0 1 0] Input Action Functions that can be assigned to different key in the Menu System's Key Binding settings
  (:`Pressed`
    (`KismetSystemLibrary.PrintString` "Inventory")))

(event `InputAction|IA_MenuSys_Custom1`
  (params (Key :type "Key Structure"))
  ;[0 1 0] Input Action Functions that can be assigned to different key in the Menu System's Key Binding settings
  (:`Pressed`
    (`KismetSystemLibrary.PrintString` "Custom1")))

(event `Key|Escape`
  (params (Key :type "Key Structure"))
  ;[0 1 0] Use Escape Key for Production Deployment
)

(event `Key|Tab`
  (params (Key :type "Key Structure"))
  (bind _returnvalue (`GameplayStatics.GetPlayerController` 0))
  ;[0 1 0] Use Tab Key when Debugging in editor
  (:`Pressed`
    ;[0 1 0] Invoke the In-Game Pause Menu when player presses the In-Game Pause Menu key (NOTE: Disconnect the Escape Key when developing/playing in Editor)
    (`/Engine/EditorBlueprintResources/StandardMacros.IsValid` (`self.InGamePauseMenuRef`)
      (:`Is Valid`
        _)
      (:`Is Not Valid`
        (bind _returnvalue_2 (`|CreateWidget` "/Game/DZG_MenuSystemV1/UI/WBP_InGamePauseMenu.WBP_InGamePauseMenu_C" _returnvalue))
        (bind _output_get (set `self.InGamePauseMenuRef` _returnvalue_2))))
    (`UserWidget.AddToViewport` _output_get 0)
    (`WidgetBlueprintLibrary.SetInputMode_UIOnlyEx` _returnvalue null)
    (set `PlayerController.bShowMouseCursor` true _returnvalue)
    (`GameplayStatics.SetGamePaused` true)))

(fn `UserConstructionScript`)